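; Bubble projectile actor that notifies interactable targets on impact and destroys itself after any hit.
; Targets implementing the BubbleInteract interface receive InteractMessage, and the projectile calls ProjectileHit.
; An interface hit also plays a pop sound and briefly flashes a hit marker widget, guarded by a boolean, with a short delay before removal.
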(event `self.ReceiveHit`
  (params (MyComp :type "PrimitiveComponent Object Reference") (Other :type "Actor Object Reference") (OtherComp :type "PrimitiveComponent Object Reference") (bSelfMoved :type Boolean) (HitLocation :type "Vector Structure") (HitNormal :type "Vector Structure") (NormalImpulse :type "Vector Structure") (Hit :type "HitResult Structure (by ref)"))
  (if (`KismetSystemLibrary.DoesImplementInterface` Other "/Game/Blueprints/BubbleInteract.BubbleInteract_C")
    (message `/Game/Blueprints/BubbleInteract.Interact` Other)
    (`self.ProjectileHit`)
    (if (not (`self.HitMarker`))
      (bind _returnvalue (`|CreateWidget` "/Game/UI/WB_HitMarker.WB_HitMarker_C"))
      (`UserWidget.AddToViewport` _returnvalue 0)
      (set `self.HitMarker` true)
      (`GameplayStatics.PlaySoundAtLocation` "/Game/Audio/Sound_Effects/Pop.Pop" HitLocation (struct) 1.0 1.0 0.0 null null null null)
      (`KismetSystemLibrary.Delay` 0.017)
      (`Widget.RemoveFromParent` _returnvalue)
      (set `self.HitMarker` false))
    (`self.K2_DestroyActor`)
    (else
      (`self.K2_DestroyActor`))))

(fn `UserConstructionScript`)