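; Parent Blueprint for enemy fish that accumulate a bubble and die when its size reaches their Health.
; BubbleIncrease and BubbleDecrease adjust CurrentBubbleSize and refresh the Bubble's uniform scale, with only increases checking for death.
; The scale lerps from zero toward MaxBubleSize over a fixed 100-unit range, independent of Health and without clamping.
; Death is an empty function here.
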(fn `BubbleDecrease`
  (params (Value :type "Float (double-precision)"))
  (set `self.CurrentBubbleSize` (- (`self.CurrentBubbleSize`) Value))
  (`self.UpdateBubbleVisual`))

(fn `BubbleIncrease`
  (params (Value :type "Float (double-precision)"))
  (set `self.CurrentBubbleSize` (+ (`self.CurrentBubbleSize`) Value))
  (`self.UpdateBubbleVisual`)
  (if (>= (`self.CurrentBubbleSize`) (`self.Health`))
    (`self.Death`)))

(fn `Death`)

(fn `UpdateBubbleVisual`
  (bind _returnvalue (`KismetMathLibrary.Lerp` 0.0 (`self.MaxBubleSize`) (/ (`self.CurrentBubbleSize`) 100.0)))
  (`SceneComponent.SetRelativeScale3D` (`self.Bubble`) (`KismetMathLibrary.MakeVector` _returnvalue _returnvalue _returnvalue)))

(fn `UserConstructionScript`)