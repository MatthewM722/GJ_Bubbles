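; Child Blueprint for a swordfish enemy that defines what happens when it dies.
; Death disables collision, sets Dead and hides the health bar.
; It then reuses projectile movement for a bubble-rising effect, capping speed, freeing rotation from velocity and homing on a Scene component.
; The actor destroys itself after a delay, but only if the player pawn casts to Pawn_Sharkfish.
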(event `self.Death`
  (`PrimitiveComponent.SetCollisionEnabled` (`self.Collision`) "NoCollision")
  (set `self.Dead` true)
  (`SceneComponent.SetVisibility` (`self.Health Bar`) false false)
  ; Bubble Rising
  (set `ProjectileMovementComponent.bRotationFollowsVelocity` false (`self.ProjectileMovement`))
  (set `ProjectileMovementComponent.MaxSpeed` 400.0 (`self.ProjectileMovement`))
  (set `ProjectileMovementComponent.HomingTargetComponent` (`self.Scene`) (`self.ProjectileMovement`))
  (cast `/Game/Character/Pawn_Sharkfish` (`GameplayStatics.GetPlayerPawn` 0))
  (`KismetSystemLibrary.Delay` 6.0)
  (`self.K2_DestroyActor`))

(fn `UserConstructionScript`
  (`parent.UserConstructionScript`))