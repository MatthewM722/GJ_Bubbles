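; Mortar shark enemy, a child Blueprint that periodically launches Child_Swordfish actors at the player.
; Tick feeds a Delay randomized around FireDelay by RandomnessRange, acting as a repeating fire timer.
; Each shot spawns at the GunBarrel location, adjusting for collisions but always spawning.
; The spawned swordfish then receives the Arrow component of the player's Pawn_Sharkfish as its Target.
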(event `self.ReceiveTick`
  (params (DeltaSeconds :type "Float (single-precision)"))
  (`KismetSystemLibrary.Delay` (`KismetMathLibrary.RandomFloatInRange` (- (`self.FireDelay`) (`self.RandomnessRange`)) (+ (`self.FireDelay`) (`self.RandomnessRange`))))
  (bind _returnvalue (`|SpawnActorFromClass` "/Game/Blueprints/Enemies/Child_Swordfish.Child_Swordfish_C" (`KismetMathLibrary.MakeTransform` (`SceneComponent.K2_GetComponentLocation` (`self.GunBarrel`))) "AdjustIfPossibleButAlwaysSpawn" "MultiplyWithRoot" null null))
  (bind _aspawn_sharkfish (cast `/Game/Character/Pawn_Sharkfish` (`GameplayStatics.GetPlayerPawn` 0)))
  (set `/Game/Blueprints/Enemies/Parent_EnemyFish.Target` (`/Game/Character/Pawn_Sharkfish.Arrow` _aspawn_sharkfish) _returnvalue))

(fn `UserConstructionScript`
  (`parent.UserConstructionScript`))