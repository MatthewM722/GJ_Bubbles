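; Child_MOAB is an enemy fish variant that splits into three new enemies when it is destroyed, whatever the cause.
; Its Destroyed event runs a sequence that force-spawns one actor at the SMFish mesh location and two Parent_EnemyFish at opposite diagonal offsets from it.
; Each spawned enemy inherits the destroyed actor's Target.
; The construction script only calls the parent's.
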(event `self.ReceiveDestroyed`
  (`|ExecutionSequence`
    (:`then_0`
      (bind _returnvalue (`|SpawnActorFromClass` "/Game/Blueprints/Enemies/Parent_EnemyFish.Parent_EnemyFish_C" (`KismetMathLibrary.MakeTransform` (`SceneComponent.K2_GetComponentLocation` (`self.SM_Fish`))) "AlwaysSpawn" "MultiplyWithRoot" null null))
      (set `/Game/Blueprints/Enemies/Parent_EnemyFish.Target` (`self.Target`) _returnvalue))
    (:`then_1`
      (bind _returnvalue_2 (`|SpawnActorFromClass` "/Game/Blueprints/Enemies/Parent_EnemyFish.Parent_EnemyFish_C" (`KismetMathLibrary.MakeTransform` (+ (`SceneComponent.K2_GetComponentLocation` (`self.SM_Fish`)) (140.0 120.0 160.0))) "AlwaysSpawn" "MultiplyWithRoot" null null))
      (set `/Game/Blueprints/Enemies/Parent_EnemyFish.Target` (`self.Target`) _returnvalue_2))
    (:`then_2`
      (bind _returnvalue_3 (`|SpawnActorFromClass` "/Game/Blueprints/Enemies/Parent_EnemyFish.Parent_EnemyFish_C" (`KismetMathLibrary.MakeTransform` (+ (`SceneComponent.K2_GetComponentLocation` (`self.SM_Fish`)) (-140.0 -120.0 -160.0))) "AlwaysSpawn" "MultiplyWithRoot" null null))
      (set `/Game/Blueprints/Enemies/Parent_EnemyFish.Target` (`self.Target`) _returnvalue_3))))

(fn `UserConstructionScript`
  (`parent.UserConstructionScript`))