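; Wave manager that runs fifteen enemy fish waves, damages the player when fish pass the gate, and updates the HUD.
; NewWave picks the current wave, which sets the enemy count and plays a Timeline whose event tracks trigger spawn functions.
; Each fish spawns at a random point with a random target and a manager reference.
; When the count reaches zero, it advances the wave, clears FishInLevel actors and opens the submenu.
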(event `Update Wave`
  (bind _aspawn_sharkfish (cast `/Game/Character/Pawn_Sharkfish` (`GameplayStatics.GetPlayerPawn` 0)))
  (`/Game/UI/WB_HUD.Update Wave` (`/Game/Character/Pawn_Sharkfish.Reference_HUD` _aspawn_sharkfish) (`self.CurrentWave`)))

(event `Update Enemy Left Text`
  ; Updates HUD
  (bind _aspawn_sharkfish (cast `/Game/Character/Pawn_Sharkfish` (`GameplayStatics.GetPlayerPawn` 0)))
  (`/Game/UI/WB_HUD.Update Enemies Left` (`/Game/Character/Pawn_Sharkfish.Reference_HUD` _aspawn_sharkfish) (`self.EnemiesLeft`)))

(event `OpenSubmenu`
  (bind _returnvalue (`|CreateWidget` "/Game/UI/WB_SubMenu.WB_SubMenu_C"))
  (`UserWidget.AddToViewport` _returnvalue 0)
  (bind _aspawn_sharkfish (cast `/Game/Character/Pawn_Sharkfish` (`GameplayStatics.GetPlayerPawn` 0)))
  (set `Widget.Visibility` "Hidden" (`/Game/UI/WB_HUD.Crosshair` (`/Game/Character/Pawn_Sharkfish.Reference_HUD` _aspawn_sharkfish)))
  (bind _asplayer_controller (cast `PlayerController` (`GameplayStatics.GetPlayerController` 0)))
  (`WidgetBlueprintLibrary.SetInputMode_UIOnlyEx` _asplayer_controller _returnvalue)
  (set `PlayerController.bShowMouseCursor` true _asplayer_controller)
  (`PlayerController.SetViewTargetWithBlend` _asplayer_controller (`self.SubmenuCamera`) 0.3 "VTBlend_Linear" 0.0 false))

(event `Remove Enemy`
  ; Enemy Counter
  (bind _aspawn_sharkfish (cast `/Game/Character/Pawn_Sharkfish` (`GameplayStatics.GetPlayerPawn` 0)))
  (if (not (`/Game/Character/Pawn_Sharkfish.Dead` _aspawn_sharkfish))
    (set `self.EnemiesLeft` (- (`self.EnemiesLeft`) 1))
    (`self.Update Enemy Left Text`)
    (if (<= (`self.EnemiesLeft`) 0)
      (`/Engine/EditorBlueprintResources/StandardMacros.IncrementInt` (`self.CurrentWave`)
        (:`  `
          (`KismetSystemLibrary.Delay` 2.0)
          (if true
            (for _array_element (`self.FishInLevel`)
              (`self.K2_DestroyActor` _array_element))
            (`KismetArrayLibrary.Array_Clear` (`self.FishInLevel`)))
          (`self.OpenSubmenu`))))))

(event `self.CollisionBox.OnComponentBeginOverlap`
  (params (OverlappedComponent :type "PrimitiveComponent Object Reference") (OtherActor :type "Actor Object Reference") (OtherComp :type "PrimitiveComponent Object Reference") (OtherBodyIndex :type Integer) (bFromSweep :type Boolean) (SweepResult :type "HitResult Structure (by ref)"))
  ; Removes health from player when fish pass the gate
  (bind _asparent_enemy_fish (cast `/Game/Blueprints/Enemies/Parent_EnemyFish` OtherActor))
  (bind _aspawn_sharkfish (cast `/Game/Character/Pawn_Sharkfish` (`GameplayStatics.GetPlayerPawn` 0)))
  (`/Game/Character/Pawn_Sharkfish.DecreaseHealth` _aspawn_sharkfish (`/Game/Blueprints/Enemies/Parent_EnemyFish.Damage` _asparent_enemy_fish))
  (if (`/Game/Blueprints/Enemies/Parent_EnemyFish.CountsAsEnemy` _asparent_enemy_fish)
    (`self.Remove Enemy`))
  (`self.K2_DestroyActor` _asparent_enemy_fish))

(event `Wave1`
  ; Wave 1
  (set `self.EnemiesLeft` 4)
  (`self.Update Enemy Left Text`)
  (`Timeline|Wave 1`
    (:`Standard Fish`
      (`self.Spawn_StandardFish`))
    (:`School`
      (`self.Spawn_School`))))

(event `Wave2`
  ; Wave 2
  (set `self.EnemiesLeft` 8)
  (`self.Update Enemy Left Text`)
  (`Timeline|Wave 2`
    (:`Standard Fish`
      (`self.Spawn_StandardFish`))
    (:`School`
      (`self.Spawn_School`))
    (:`Catfish`
      (`self.Spawn_Catfish`))))

(event `New Wave`
  ; Wave Selector
  (`self.Update Wave`)
  (switch `int` (`self.CurrentWave`)
    (:`1`
      (`self.Wave1`))
    (:`2`
      (`self.Wave2`))
    (:`3`
      (`self.Wave3`))
    (:`4`
      (`self.Wave4`))
    (:`5`
      (`self.Wave5`))
    (:`6`
      (`self.Wave6`))
    (:`7`
      (`self.Wave7`))
    (:`8`
      (`self.Wave8`))
    (:`9`
      (`self.Wave9`))
    (:`10`
      (`self.Wave10`))
    (:`11`
      (`self.Wave11`))
    (:`12`
      (`self.Wave12`))
    (:`13`
      (`self.Wave13`))
    (:`14`
      (`self.Wave14`))
    (:`15`
      (`self.Wave15`))))

(event `Wave3`
  ; Wave 3
  (set `self.EnemiesLeft` 5)
  (`self.Update Enemy Left Text`)
  (`Timeline|Wave 3`
    (:`Standard Fish`
      (`self.Spawn_StandardFish`))
    (:`School`
      (`self.Spawn_School`))
    (:`Hammerhead`
      (`self.Spawn_Hammerhead`))
    (:`Catfish`
      (`self.Spawn_Catfish`))))

(event `Wave4`
  (set `self.EnemiesLeft` 8)
  (`self.Update Enemy Left Text`)
  (`Timeline|Wave 4`
    (:`Standard Fish`
      (`self.Spawn_StandardFish`))
    (:`School`
      (`self.Spawn_School`))
    (:`Hammerhead`
      (`self.Spawn_Hammerhead`))))

(event `Wave5`
  (set `self.EnemiesLeft` 2)
  (`self.Update Enemy Left Text`)
  (`Timeline|Wave 5`
    (:`Mortar Shark`
      (`self.Spawn_MortarShark`))))

(event `Wave6`
  (set `self.EnemiesLeft` 7)
  (`self.Update Enemy Left Text`)
  (`Timeline|Wave 6`
    (:`Standard Fish`
      (`self.Spawn_StandardFish`))
    (:`School`
      (`self.Spawn_School`))
    (:`Hammerhead`
      (`self.Spawn_Hammerhead`))
    (:`Mortar Shark`
      (`self.Spawn_MortarShark`))
    (:`Catfish`
      (`self.Spawn_Catfish`))))

(event `Wave7`
  (set `self.EnemiesLeft` 9)
  (`self.Update Enemy Left Text`)
  (`Timeline|Wave 7`
    (:`Standard Fish`
      (`self.Spawn_StandardFish`))
    (:`School`
      (`self.Spawn_School`))
    (:`Hammerhead`
      (`self.Spawn_Hammerhead`))
    (:`Mortar Shark`
      (`self.Spawn_MortarShark`))))

(event `Wave8`
  (set `self.EnemiesLeft` 3)
  (`self.Update Enemy Left Text`)
  (`Timeline|Wave 8`
    (:`Mortar Shark`
      (`self.Spawn_MortarShark`))
    (:`Anglerfish`
      (`self.Spawn_Anglerfish`))))

(event `Wave9`
  (set `self.EnemiesLeft` 8)
  (`self.Update Enemy Left Text`)
  (`Timeline|Wave 9`
    (:`Standard Fish`
      (`self.Spawn_StandardFish`))
    (:`School`
      (`self.Spawn_School`))
    (:`Hammerhead`
      (`self.Spawn_Hammerhead`))
    (:`Anglerfish`
      (`self.Spawn_Anglerfish`))))

(event `Wave10`
  (set `self.EnemiesLeft` 1)
  (`self.Update Enemy Left Text`)
  (`Timeline|Wave 10`
    (:`MOAB`
      (`self.Spawn_MOAB`))))

(event `Wave11`
  (set `self.EnemiesLeft` 8)
  (`self.Update Enemy Left Text`)
  (`Timeline|Wave 11`
    (:`Standard Fish`
      (`self.Spawn_StandardFish`))
    (:`School`
      (`self.Spawn_School`))
    (:`Hammerhead`
      (`self.Spawn_Hammerhead`))
    (:`Anglerfish`
      (`self.Spawn_Anglerfish`))
    (:`Mortar Shark`
      (`self.Spawn_MortarShark`))
    (:`Catfish`
      (`self.Spawn_Catfish`))
    (:`Moab`
      (`self.Spawn_MOAB`))))

(event `Wave12`
  (set `self.EnemiesLeft` 10)
  (`self.Update Enemy Left Text`)
  (`Timeline|Wave 12`
    (:`Standard Fish`
      (`self.Spawn_StandardFish`))
    (:`School`
      (`self.Spawn_School`))
    (:`Hammerhead`
      (`self.Spawn_Hammerhead`))
    (:`Anglerfish`
      (`self.Spawn_Anglerfish`))
    (:`Mortar Shark`
      (`self.Spawn_MortarShark`))
    (:`Catfish`
      (`self.Spawn_Catfish`))
    (:`Moab`
      (`self.Spawn_MOAB`))))

(event `Wave13`
  (set `self.EnemiesLeft` 6)
  (`self.Update Enemy Left Text`)
  (`Timeline|Wave 13`
    (:`Standard Fish`
      (`self.Spawn_StandardFish`))
    (:`School`
      (`self.Spawn_School`))
    (:`Hammerhead`
      (`self.Spawn_Hammerhead`))
    (:`Anglerfish`
      (`self.Spawn_Anglerfish`))
    (:`Mortar Shark`
      (`self.Spawn_MortarShark`))
    (:`Catfish`
      (`self.Spawn_Catfish`))
    (:`Moab`
      (`self.Spawn_MOAB`))))

(event `Wave14`
  (set `self.EnemiesLeft` 15)
  (`self.Update Enemy Left Text`)
  (`Timeline|Wave 14`
    (:`Standard Fish`
      (`self.Spawn_StandardFish`))
    (:`School`
      (`self.Spawn_School`))
    (:`Hammerhead`
      (`self.Spawn_Hammerhead`))
    (:`Anglerfish`
      (`self.Spawn_Anglerfish`))
    (:`Mortar Shark`
      (`self.Spawn_MortarShark`))
    (:`Catfish`
      (`self.Spawn_Catfish`))
    (:`Moab`
      (`self.Spawn_MOAB`))))

(event `Wave15`
  (set `self.EnemiesLeft` 26)
  (`self.Update Enemy Left Text`)
  (`Timeline|Wave 15`
    (:`Standard Fish`
      (`self.Spawn_StandardFish`))
    (:`School`
      (`self.Spawn_School`))
    (:`Hammerhead`
      (`self.Spawn_Hammerhead`))
    (:`Anglerfish`
      (`self.Spawn_Anglerfish`))
    (:`Mortar Shark`
      (`self.Spawn_MortarShark`))
    (:`Catfish`
      (`self.Spawn_Catfish`))
    (:`Moab`
      (`self.Spawn_MOAB`))))

(fn `GainRandomTarget`
  (returns (Target :type "ArrowComponent Object Reference"))
  (bind _target (`self.RandomTarget`))
  (return _target))

(fn `RandomTarget`
  (returns (Target :type "ArrowComponent Object Reference"))
  (switch `int` (`KismetMathLibrary.RandomIntegerInRange` 0 3)
    (:`0`
      (return (`self.Target1`)))
    (:`1`
      (return (`self.Target2`)))
    (:`2`
      (return (`self.Target3`)))
    (:`3`
      (return (`self.Target4`)))))

(fn `Spawn_Anglerfish`
  (bind _returnvalue_location (`KismetMathLibrary.BreakTransform` (`self.GetTransform` (`|GetArrayItem` (`self.SpawnPoints`) (`KismetMathLibrary.RandomInteger` (`KismetArrayLibrary.Array_Length` (`self.SpawnPoints`)))))))
  (bind _returnvalue (`|SpawnActorFromClass` "/Game/Blueprints/Enemies/Child_AnglerFish.Child_Anglerfish_C" (`KismetMathLibrary.MakeTransform` _returnvalue_location (struct) (2.0 2.0 2.0)) "AdjustIfPossibleButAlwaysSpawn" "MultiplyWithRoot" null null))
  (bind _target (`self.RandomTarget`))
  (set `/Game/Blueprints/Enemies/Parent_EnemyFish.Target` _target _returnvalue)
  (set `/Game/Blueprints/Enemies/Parent_EnemyFish.Reference_WaveManager` self _returnvalue))

(fn `Spawn_Catfish`
  (bind _returnvalue_location (`KismetMathLibrary.BreakTransform` (`self.GetTransform` (`|GetArrayItem` (`self.SpawnPoints`) (`KismetMathLibrary.RandomInteger` (`KismetArrayLibrary.Array_Length` (`self.SpawnPoints`)))))))
  (bind _returnvalue (`|SpawnActorFromClass` "/Game/Blueprints/Enemies/Child_Catfish.Child_Catfish_C" (`KismetMathLibrary.MakeTransform` _returnvalue_location (struct) (2.0 2.0 2.0)) "AdjustIfPossibleButAlwaysSpawn" "MultiplyWithRoot" null null))
  (bind _target (`self.RandomTarget`))
  (set `/Game/Blueprints/Enemies/Parent_EnemyFish.Target` _target _returnvalue)
  (set `/Game/Blueprints/Enemies/Parent_EnemyFish.Reference_WaveManager` self _returnvalue))

(fn `Spawn_Hammerhead`
  (bind _returnvalue_location (`KismetMathLibrary.BreakTransform` (`self.GetTransform` (`|GetArrayItem` (`self.SpawnPoints`) (`KismetMathLibrary.RandomInteger` (`KismetArrayLibrary.Array_Length` (`self.SpawnPoints`)))))))
  (bind _returnvalue (`|SpawnActorFromClass` "/Game/Blueprints/Enemies/Child_Hammerhead.Child_Hammerhead_C" (`KismetMathLibrary.MakeTransform` _returnvalue_location (struct) (2.0 2.0 2.0)) "AdjustIfPossibleButAlwaysSpawn" "MultiplyWithRoot" null null))
  (bind _target (`self.RandomTarget`))
  (set `/Game/Blueprints/Enemies/Parent_EnemyFish.Target` _target _returnvalue)
  (set `/Game/Blueprints/Enemies/Parent_EnemyFish.Reference_WaveManager` self _returnvalue))

(fn `Spawn_MOAB`
  (bind _returnvalue_location (`KismetMathLibrary.BreakTransform` (`self.GetTransform` (`|GetArrayItem` (`self.SpawnPoints`) (`KismetMathLibrary.RandomInteger` (`KismetArrayLibrary.Array_Length` (`self.SpawnPoints`)))))))
  (bind _returnvalue (`|SpawnActorFromClass` "/Game/Blueprints/Enemies/Child_MOAB.Child_MOAB_C" (`KismetMathLibrary.MakeTransform` _returnvalue_location (struct) (1.5 1.5 1.5)) "AlwaysSpawn" "MultiplyWithRoot" null null))
  (bind _target (`self.RandomTarget`))
  (set `/Game/Blueprints/Enemies/Parent_EnemyFish.Target` _target _returnvalue)
  (set `/Game/Blueprints/Enemies/Parent_EnemyFish.Reference_WaveManager` self _returnvalue))

(fn `Spawn_MortarShark`
  (bind _returnvalue_location (`KismetMathLibrary.BreakTransform` (`self.GetTransform` (`|GetArrayItem` (`self.SpawnPoints`) (`KismetMathLibrary.RandomInteger` (`KismetArrayLibrary.Array_Length` (`self.SpawnPoints`)))))))
  (bind _returnvalue (`|SpawnActorFromClass` "/Game/Blueprints/Enemies/Child_MortarShark.Child_MortarShark_C" (`KismetMathLibrary.MakeTransform` _returnvalue_location (struct) (2.0 2.0 2.0)) "AdjustIfPossibleButAlwaysSpawn" "MultiplyWithRoot" null null))
  (bind _target (`self.RandomTarget`))
  (set `/Game/Blueprints/Enemies/Parent_EnemyFish.Target` _target _returnvalue)
  (set `/Game/Blueprints/Enemies/Parent_EnemyFish.Reference_WaveManager` self _returnvalue))

(fn `Spawn_School`
  (bind _returnvalue_location (`KismetMathLibrary.BreakTransform` (`self.GetTransform` (`|GetArrayItem` (`self.SpawnPoints`) (`KismetMathLibrary.RandomInteger` (`KismetArrayLibrary.Array_Length` (`self.SpawnPoints`)))))))
  (bind _returnvalue (`|SpawnActorFromClass` "/Game/Blueprints/Enemies/Child_School.Child_School_C" (`KismetMathLibrary.MakeTransform` _returnvalue_location (struct) (2.0 2.0 2.0)) "AdjustIfPossibleButAlwaysSpawn" "MultiplyWithRoot" null null))
  (bind _target (`self.RandomTarget`))
  (set `/Game/Blueprints/Enemies/Parent_EnemyFish.Target` _target _returnvalue)
  (set `/Game/Blueprints/Enemies/Parent_EnemyFish.Reference_WaveManager` self _returnvalue))

(fn `Spawn_StandardFish`
  (bind _returnvalue_location (`KismetMathLibrary.BreakTransform` (`self.GetTransform` (`|GetArrayItem` (`self.SpawnPoints`) (`KismetMathLibrary.RandomInteger` (`KismetArrayLibrary.Array_Length` (`self.SpawnPoints`)))))))
  (bind _returnvalue (`|SpawnActorFromClass` "/Game/Blueprints/Enemies/Child_StandardFish.Child_StandardFish_C" (`KismetMathLibrary.MakeTransform` _returnvalue_location (struct) (1.5 1.5 1.5)) "AdjustIfPossibleButAlwaysSpawn" "MultiplyWithRoot" null null))
  (bind _target (`self.RandomTarget`))
  (set `/Game/Blueprints/Enemies/Parent_EnemyFish.Target` _target _returnvalue)
  (set `/Game/Blueprints/Enemies/Parent_EnemyFish.Reference_WaveManager` self _returnvalue))

(fn `UserConstructionScript`)