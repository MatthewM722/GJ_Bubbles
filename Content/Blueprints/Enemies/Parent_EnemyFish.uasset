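; Base enemy fish that homes toward a target via ProjectileMovement and is defeated by being encased in a growing bubble.
; Damage adds to bubble health, scaling the bubble and updating a camera-facing health bar, which reads the value before each hit is added.
; At full health, Death retargets homing for the bubble rise, awards player XP, notifies the wave manager and destroys the actor after a delay.
; BubbleDecrease and GainRandomTarget are non-functional stubs.
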(event `/Game/Blueprints/BI_BubbleInteract.DamageEnemy`
  (params (Amount :type "Float (double-precision)"))
  (`self.BubbleIncrease` Amount))

(event `self.ReceiveBeginPlay`
  (set `ProjectileMovementComponent.InitialSpeed` (`self.Speed`) (`self.ProjectileMovement`))
  (set `ProjectileMovementComponent.MaxSpeed` (`self.Speed`) (`self.ProjectileMovement`))
  (`KismetSystemLibrary.Delay` 0.1)
  (set `ProjectileMovementComponent.HomingTargetComponent` (`self.Target`) (`self.ProjectileMovement`)))

(event `Death`
  (`PrimitiveComponent.SetCollisionEnabled` (`self.Collision`) "NoCollision")
  (set `self.Dead` true)
  (`SceneComponent.SetVisibility` (`self.Health Bar`) false false)
  ; Bubble Rising
  (set `ProjectileMovementComponent.bRotationFollowsVelocity` false (`self.ProjectileMovement`))
  (set `ProjectileMovementComponent.MaxSpeed` 400.0 (`self.ProjectileMovement`))
  (set `ProjectileMovementComponent.HomingTargetComponent` (`self.Scene`) (`self.ProjectileMovement`))
  (bind _aspawn_sharkfish (cast `/Game/Character/Pawn_Sharkfish` (`GameplayStatics.GetPlayerPawn` 0)))
  (`/Game/Character/Pawn_Sharkfish.XPGain` _aspawn_sharkfish (`self.XP_Rewarded`))
  (`/Game/Blueprints/Enemies/BP_WaveManager.Remove Enemy` (`self.Reference_WaveManager`))
  (`KismetSystemLibrary.Delay` 6.0)
  (`self.K2_DestroyActor`))

(fn `BubbleDecrease`
  (set `self.CurrentBubbleHealth` (- (`self.CurrentBubbleHealth`) 0.0))
  (`self.UpdateBubbleVisual`))

(fn `BubbleIncrease`
  (params (Value :type "Float (double-precision)"))
  (bind _health (`self.Health`))
  (bind _health_bar (`self.Health Bar`))
  ;[0.7569 0.1255 0.1686] Health Bar
  (bind _aswb_enemy_health_bar (cast `/Game/UI/WB_EnemyHealthBar` (`WidgetComponent.GetWidget` (`self.Health Bar`))))
  (`ProgressBar.SetPercent` (`/Game/UI/WB_EnemyHealthBar.EnemyHealthBarWidget` _aswb_enemy_health_bar) (/ (stale _output_get) _health))
  (`SceneComponent.K2_SetWorldRotation` _health_bar (`KismetMathLibrary.FindLookAtRotation` (`SceneComponent.K2_GetComponentLocation` _health_bar) (`SceneComponent.K2_GetComponentLocation` (`PlayerCameraManager.TransformComponent` (`GameplayStatics.GetPlayerCameraManager` 0)))) false false)
  (if (not (`self.Dead`))
    (bind _output_get (set `self.CurrentBubbleHealth` (+ (`self.CurrentBubbleHealth`) Value)))
    (`self.UpdateBubbleVisual`)
    (if (>= (`self.CurrentBubbleHealth`) _health)
      (`self.Death`))))

(fn `GainRandomTarget`
  (returns (Target :type "ArrowComponent Object Reference"))
  (return null))

(fn `UpdateBubbleVisual`
  (bind _returnvalue (`KismetMathLibrary.Lerp` 0.0 (`self.MaxBubbleSize`) (/ (`self.CurrentBubbleHealth`) (`self.Health`))))
  (`SceneComponent.SetRelativeScale3D` (`self.Bubble`) (`KismetMathLibrary.MakeVector` _returnvalue _returnvalue _returnvalue)))

(fn `UserConstructionScript`)