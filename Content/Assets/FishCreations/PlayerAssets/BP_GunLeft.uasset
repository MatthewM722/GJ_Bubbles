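; Left-hand gun actor that fires bubble projectiles and turns toward the player's camera aim point.
; GunLeftFire spawns a randomly scaled BubbleProjectile at the Gun_L socket, then line-traces forward from the camera.
; The mesh then interpolates toward the hit location using a fixed delta time, so aim only updates when firing, after the spawn.
; Tick gathers all live bubbles every frame as the trace's ignore list.
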(event `self.ReceiveBeginPlay`)

(event `GunLeftFire`
  (bind (_returnvalue_location _returnvalue_rotation) (`KismetMathLibrary.BreakTransform` (`SceneComponent.GetSocketTransform` (`self.SM_GunLeft`) "Gun_L" "RTS_World")))
  (bind _returnvalue (`self.K2_GetActorLocation` (`GameplayStatics.GetPlayerCameraManager` 0)))
  (`|SpawnActorFromClass` "/Game/Blueprints/BubbleProjectile.BubbleProjectile_C" (`KismetMathLibrary.MakeTransform` _returnvalue_location _returnvalue_rotation (`KismetMathLibrary.Conv_DoubleToVector` (`KismetMathLibrary.RandomFloatInRange` 0.8 2.0))) "Undefined" "MultiplyWithRoot" null null)
  (bind _outhit (`KismetSystemLibrary.LineTraceSingle` _returnvalue (+ _returnvalue (* (`self.GetActorForwardVector` (`GameplayStatics.GetPlayerCameraManager` 0)) (100000.0 100000.0 100000.0))) "TraceTypeQuery1" false (stale `self.ReceiveTick` _outactors)))
  (`SceneComponent.K2_SetWorldRotation` (`self.SM_GunLeft`) (`KismetMathLibrary.RInterpTo` (`SceneComponent.GetSocketRotation` (`self.SM_GunLeft`) "Gun_L") (`KismetMathLibrary.FindLookAtRotation` (`SceneComponent.GetSocketLocation` (`self.SM_GunLeft`) "Gun_L") (`.Location` (`GameplayStatics.BreakHitResult` _outhit))) 0.0166 30.0) false false))

(event `self.ReceiveTick`
  (params (DeltaSeconds :type "Float (single-precision)"))
  (bind _outactors (`GameplayStatics.GetAllActorsOfClass` "/Game/Blueprints/BubbleProjectile.BubbleProjectile_C")))

(fn `UserConstructionScript`)