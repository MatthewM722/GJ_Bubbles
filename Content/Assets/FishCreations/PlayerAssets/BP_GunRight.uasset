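; BP_GunRight is the player's right-hand bubble gun, firing when its GunRightFire event is called.
; It spawns a randomly scaled BubbleProjectile at the Gun_R socket and passes it the damage.
; After spawning, it traces from the camera, ignoring bubbles, and interpolates the gun mesh toward the hit location with a fixed timestep.
; Aim only updates on firing, so each correction affects subsequent shots.
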(event `GunRightFire`
  (params (Damage :type "Float (double-precision)"))
  (bind (_returnvalue_location _returnvalue_rotation) (`KismetMathLibrary.BreakTransform` (`SceneComponent.GetSocketTransform` (`self.SM_GunRight`) "Gun_R" "RTS_World")))
  (bind _returnvalue (`self.K2_GetActorLocation` (`GameplayStatics.GetPlayerCameraManager` 0)))
  (bind _returnvalue_2 (`|SpawnActorFromClass` "/Game/Blueprints/BubbleProjectile.BubbleProjectile_C" (`KismetMathLibrary.MakeTransform` _returnvalue_location _returnvalue_rotation (`KismetMathLibrary.Conv_DoubleToVector` (`KismetMathLibrary.RandomFloatInRange` 0.8 2.0))) "Undefined" "MultiplyWithRoot" null null))
  (set `/Game/Blueprints/BubbleProjectile.Damage` Damage _returnvalue_2)
  (bind _outactors (`GameplayStatics.GetAllActorsOfClass` "/Game/Blueprints/BubbleProjectile.BubbleProjectile_C"))
  (bind _outhit (`KismetSystemLibrary.LineTraceSingle` _returnvalue (+ _returnvalue (* (`self.GetActorForwardVector` (`GameplayStatics.GetPlayerCameraManager` 0)) (100000.0 100000.0 100000.0))) "TraceTypeQuery1" false _outactors))
  (`SceneComponent.K2_SetWorldRotation` (`self.SM_GunRight`) (`KismetMathLibrary.RInterpTo` (`SceneComponent.GetSocketRotation` (`self.SM_GunRight`) "Gun_R") (`KismetMathLibrary.FindLookAtRotation` (`SceneComponent.GetSocketLocation` (`self.SM_GunRight`) "Gun_R") (`.Location` (`GameplayStatics.BreakHitResult` _outhit))) 0.0166 30.0) false false))

(fn `UserConstructionScript`)