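; BP_Turret is an automatic turret that aims and shoots bubble projectiles at the nearest actor tagged Enemy.
; A looping timer started on BeginPlay rescans all tagged actors and picks the closest by distance.
; When a valid target is found, it snaps the turret mesh to face it, spawns a BubbleProjectile at the mesh's Turret socket, then resets the search.
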(event `self.ReceiveBeginPlay`
  (`KismetSystemLibrary.K2_SetTimerDelegate` (delegate `Turret`) 0.2 true))

(event `Turret`
  (bind _returnvalue (`self.K2_GetActorLocation`))
  (bind (_returnvalue_location _returnvalue_rotation _returnvalue_scale) (`KismetMathLibrary.BreakTransform` (`SceneComponent.GetSocketTransform` (`self.SM_Turret`) "Turret" "RTS_World")))
  (bind _outactors (`GameplayStatics.GetAllActorsWithTag` "Enemy"))
  (for _array_element _outactors
    (bind _returnvalue_2 (`KismetMathLibrary.VSize` (- (`self.K2_GetActorLocation` _array_element) _returnvalue)))
    (if (< _returnvalue_2 (`self.ShortestDistance`))
      (set `self.ShortestDistance` _returnvalue_2)
      (set `self.NearestEnemy` _array_element)))
  (bind _nearestenemy (`self.NearestEnemy`)
    (:`then`
      (`SceneComponent.K2_SetWorldRotation` (`self.SM_Turret`) (`KismetMathLibrary.FindLookAtRotation` _returnvalue (`self.K2_GetActorLocation` _nearestenemy)) false false)
      (`|SpawnActorFromClass` "/Game/Blueprints/BubbleProjectile.BubbleProjectile_C" (`KismetMathLibrary.MakeTransform` _returnvalue_location _returnvalue_rotation _returnvalue_scale) "Undefined" "MultiplyWithRoot" null null)
      (set `self.ShortestDistance` 999999.0)
      (set `self.NearestEnemy` null))
    (:`else`)))

(fn `UserConstructionScript`)