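; BP_Turret2 is a purchasable turret that fires bubble projectiles at the nearest living enemy fish.
; BuyTurret starts a looping timer that scans "Enemy"-tagged actors for the closest one not dead.
; Each shot leads the target using velocity from successive positions and projectile travel time, turns the mesh, then spawns a BubbleProjectile at its "Turret" socket.
; The node passing Damage to the projectile is unconnected and never runs.
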(event `Buy Turret`
  (`KismetSystemLibrary.K2_SetTimerDelegate` (delegate `Turret`) (`self.LoopTime`) true))

(event `Turret`
  (bind _returnvalue (`self.K2_GetActorLocation`))
  (bind (_returnvalue_location _returnvalue_rotation _returnvalue_scale) (`KismetMathLibrary.BreakTransform` (`SceneComponent.GetSocketTransform` (`self.SM_Turret`) "Turret" "RTS_World")))
  (bind _outactors (`GameplayStatics.GetAllActorsWithTag` "Enemy"))
  (for _array_element _outactors
    (bind _returnvalue_2 (`KismetMathLibrary.VSize` (- (`self.K2_GetActorLocation` _array_element) _returnvalue)))
    (if (< _returnvalue_2 (`self.ShortestDistance`))
      (bind _asparent_enemy_fish (cast `/Game/Blueprints/Enemies/Parent_EnemyFish` _array_element))
      (if (not (`/Game/Blueprints/Enemies/Parent_EnemyFish.Dead` _asparent_enemy_fish))
        (set `self.ShortestDistance` _returnvalue_2)
        (set `self.NearestEnemy` _asparent_enemy_fish))))
  (bind _nearestenemy (`self.NearestEnemy`)
    (:`then`
      (bind _output_get (set `self.CurrentPosition` (`self.K2_GetActorLocation` _nearestenemy)))
      (set `self.Velocity` (/ (- _output_get (`self.PreviousPosition`)) (`self.LoopTime`)))
      (set `self.PreviousPosition` (`self.CurrentPosition`))
      (bind _output_get_2 (set `self.PredictedPosition` (+ (`self.K2_GetActorLocation` (`self.NearestEnemy`)) (* (/ (`self.ShortestDistance`) (`self.ProjectileSpeed`)) (`self.Velocity`)))))
      (`SceneComponent.K2_SetWorldRotation` (`self.SM_Turret`) (`KismetMathLibrary.RInterpTo` (`self.K2_GetActorRotation`) (`KismetMathLibrary.FindLookAtRotation` _returnvalue _output_get_2) (stale `self.ReceiveTick` DeltaSeconds) 100.0) false false)
      (bind _returnvalue_3 (`|SpawnActorFromClass` "/Game/Blueprints/BubbleProjectile.BubbleProjectile_C" (`KismetMathLibrary.MakeTransform` _returnvalue_location _returnvalue_rotation _returnvalue_scale) "Undefined" "MultiplyWithRoot" null null))
      (set `self.ShortestDistance` 999999.0)
      (set `self.NearestEnemy` null))
    (:`else`)))

(event `self.ReceiveTick`
  (params (DeltaSeconds :type "Float (single-precision)")))

(fn `UserConstructionScript`)